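; Projector actor that plays a media source and carries red, green and blue spot lights, apparently to project video in color through light functions.
; The construction script pushes shared intensity, attenuation, cone and light-function settings to all three lights.
; On BeginPlay it opens the source with configurable looping and starts playback once the media opens.
; Shadow setters on the green light are left unconnected.
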(event `self.ReceiveBeginPlay`
  (bind _mediaplayer (`self.MediaPlayer`))
  (add `MediaPlayer.OnMediaOpened` _mediaplayer (delegate `OnMediaOpened_Event_0`))
  (`MediaPlayer.OpenSource` _mediaplayer (`self.Media Source`))
  (`MediaPlayer.SetLooping` _mediaplayer (`self.Looping`)))

(event `OnMediaOpened_Event_0`
  (params (OpenedUrl :type String))
  (`MediaPlayer.Play` (`self.MediaPlayer`)))

(fn `UserConstructionScript`
  (bind _sl_green (`self.SL_GREEN`))
  (`|ExecutionSequence`
    (:`then_0`
      (`LocalLightComponent.SetIntensityUnits` _sl_green (`self.Intensity Units`))
      (`LocalLightComponent.SetIntensityUnits` (`self.SL_BLUE`) (`self.Intensity Units`))
      (`LocalLightComponent.SetIntensityUnits` (`self.SL_RED`) (`self.Intensity Units`))
      (`LightComponent.SetIntensity` _sl_green (`self.Intensity`))
      (`LightComponent.SetIntensity` (`self.SL_BLUE`) (`self.Intensity`))
      (`LightComponent.SetIntensity` (`self.SL_RED`) (`self.Intensity`))
      (`LocalLightComponent.SetAttenuationRadius` _sl_green (`self.Attenuation Radius`))
      (`LocalLightComponent.SetAttenuationRadius` (`self.SL_BLUE`) (`self.Attenuation Radius`))
      (`LocalLightComponent.SetAttenuationRadius` (`self.SL_RED`) (`self.Attenuation Radius`))
      (`SpotLightComponent.SetInnerConeAngle` _sl_green (`self.New Inner Cone Angle`))
      (`SpotLightComponent.SetInnerConeAngle` (`self.SL_BLUE`) (`self.New Inner Cone Angle`))
      (`SpotLightComponent.SetInnerConeAngle` (`self.SL_RED`) (`self.New Inner Cone Angle`))
      (`SpotLightComponent.SetOuterConeAngle` _sl_green (`self.Outer Cone Angle`))
      (`SpotLightComponent.SetOuterConeAngle` (`self.SL_BLUE`) (`self.Outer Cone Angle`))
      (`SpotLightComponent.SetOuterConeAngle` (`self.SL_RED`) (`self.Outer Cone Angle`)))
    (:`then_1`
      (`LightComponent.SetLightFunctionScale` _sl_green (`self.Light Function Scale`))
      (`LightComponent.SetLightFunctionScale` (`self.SL_BLUE`) (`self.Light Function Scale`))
      (`LightComponent.SetLightFunctionScale` (`self.SL_RED`) (`self.Light Function Scale`))
      (`LightComponent.SetLightFunctionFadeDistance` _sl_green (`self.Light Function Fade Distance`))
      (`LightComponent.SetLightFunctionFadeDistance` (`self.SL_BLUE`) (`self.Light Function Fade Distance`))
      (`LightComponent.SetLightFunctionFadeDistance` (`self.SL_RED`) (`self.Light Function Fade Distance`))
      (`LightComponent.SetLightFunctionDisabledBrightness` _sl_green (`self.Light Function Disabled Brightness`))
      (`LightComponent.SetLightFunctionDisabledBrightness` (`self.SL_BLUE`) (`self.Light Function Disabled Brightness`))
      (`LightComponent.SetLightFunctionDisabledBrightness` (`self.SL_RED`) (`self.Light Function Disabled Brightness`)))))